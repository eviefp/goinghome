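; BP_BlackHole is a black hole object that switches on a gravity-style pull for BP_ShipTest ships entering its PullArea.
; On overlap begin, it passes its root location and X scale as position and size to the ship's BlackHolePawnPull and enables it.
; On overlap end, it zeroes those values and disables the pull.
; The pull itself is not computed here, and actor scale doubles as black hole size.
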(event `self.PullArea.OnComponentBeginOverlap`
  (params (OverlappedComponent :type "PrimitiveComponent Object Reference") (OtherActor :type "Actor Object Reference") (OtherComp :type "PrimitiveComponent Object Reference") (OtherBodyIndex :type Integer) (bFromSweep :type Boolean) (SweepResult :type "HitResult Structure (by ref)"))
  (bind _returnvalue (`SceneComponent.K2_GetComponentToWorld` (`self.DefaultSceneRoot`)))
  (bind _asbp_ship_test (cast `/Game/Blueprints/Discarded/BP_ShipTest` OtherActor))
  (bind _blackholepawnpull (`/Game/Blueprints/Discarded/BP_ShipTest.BlackHolePawnPull` _asbp_ship_test))
  (set `/Game/Blueprints/Objects/BlackHolePawnPull.BlackHolePosition` (.location _returnvalue) _blackholepawnpull)
  (set `/Game/Blueprints/Objects/BlackHolePawnPull.BlackHoleSize` (.x (.scale _returnvalue)) _blackholepawnpull)
  (set `/Game/Blueprints/Objects/BlackHolePawnPull.Enabled` true _blackholepawnpull))

(event `self.PullArea.OnComponentEndOverlap`
  (params (OverlappedComponent :type "PrimitiveComponent Object Reference") (OtherActor :type "Actor Object Reference") (OtherComp :type "PrimitiveComponent Object Reference") (OtherBodyIndex :type Integer))
  (bind _asbp_ship_test (cast `/Game/Blueprints/Discarded/BP_ShipTest` OtherActor))
  (bind _blackholepawnpull (`/Game/Blueprints/Discarded/BP_ShipTest.BlackHolePawnPull` _asbp_ship_test))
  (set `/Game/Blueprints/Objects/BlackHolePawnPull.BlackHolePosition` (0.0 0.0 0.0) _blackholepawnpull)
  (set `/Game/Blueprints/Objects/BlackHolePawnPull.BlackHoleSize` 0.0 _blackholepawnpull)
  (set `/Game/Blueprints/Objects/BlackHolePawnPull.Enabled` false _blackholepawnpull))

(fn `UserConstructionScript`)