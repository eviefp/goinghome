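; BP_Asteroid is an asteroid object that shows a screen-space HUD marker following it.
; BeginPlay creates a HUDObject widget for the first player controller, centers its alignment and adds it to the viewport.
; Each Tick projects a point slightly above the actor to screen space, moves the widget there with DPI scale removed, and hides it when projection fails.
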(event `self.ReceiveBeginPlay`
  ;[1 1 1] BeginPlay - create the widget
  (bind _returnvalue (`|CreateWidget` (`self.HUDObject`) (`GameplayStatics.GetPlayerController` 0)))
  (bind _output_get (set `self.HUDInstance` _returnvalue))
  (if (`KismetSystemLibrary.IsValid` _output_get)
    (`UserWidget.SetAlignmentInViewport` _output_get (0.5 0.5))
    (`UserWidget.AddToViewport` _output_get 0)))

(event `self.ReceiveTick`
  (params (DeltaSeconds :type "Float (single-precision)"))
  (bind _hudinstance (`self.HUDInstance`))
  (bind (_screenlocation _returnvalue) (`PlayerController.ProjectWorldLocationToScreen` (`GameplayStatics.GetPlayerController` 0) (+ (`self.K2_GetActorLocation` self) (0.0 0.0 50.0)) false))
  (if (`KismetSystemLibrary.IsValid` (`self.HUDInstance`))
    (`Widget.SetVisibility` _hudinstance (select `bool` _returnvalue :`false` "Hidden" :`true` "HitTestInvisible" :!type "ESlateVisibility Enum"))
    (`UserWidget.SetPositionInViewport` _hudinstance _screenlocation true)))

(fn `UserConstructionScript`
  (`parent.UserConstructionScript`))