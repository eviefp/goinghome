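; Enemy Blueprint that detects the player's BP_Ship with a forward-facing box trigger and reports the sighting to its AI Blackboard.
; The construction script sizes and offsets the ForwardVision box from VisionDistance.
; Overlap events store the ship and toggle a flag, and Tick sets CanSeePlayer to true while that flag is set.
; Nothing here clears the key when the ship leaves.
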(event `self.ReceiveBeginPlay`
  (set `self.Overlapping` false))

(event `self.ReceiveTick`
  (params (DeltaSeconds :type "Float (single-precision)"))
  (if (`self.Overlapping`)
    (`BlackboardComponent.SetValueAsBool` (`AIBlueprintHelperLibrary.GetBlackboard` (`self.GetController`)) "CanSeePlayer" true)))

(event `self.ForwardVision.OnComponentBeginOverlap`
  (params (OverlappedComponent :type "PrimitiveComponent Object Reference") (OtherActor :type "Actor Object Reference") (OtherComp :type "PrimitiveComponent Object Reference") (OtherBodyIndex :type Integer) (bFromSweep :type Boolean) (SweepResult :type "HitResult Structure (by ref)"))
  (bind _asbp_ship (cast `/Game/Blueprints/BP_Ship` OtherActor))
  (set `self.pPlayerShip` _asbp_ship)
  (set `self.Overlapping` true))

(event `self.ForwardVision.OnComponentEndOverlap`
  (params (OverlappedComponent :type "PrimitiveComponent Object Reference") (OtherActor :type "Actor Object Reference") (OtherComp :type "PrimitiveComponent Object Reference") (OtherBodyIndex :type Integer))
  (cast `/Game/Blueprints/BP_Ship` OtherActor)
  (set `self.Overlapping` false))

(fn `UserConstructionScript`
  (bind _forwardvision (`self.ForwardVision`))
  (bind _visiondistance (`self.VisionDistance`))
  (`SceneComponent.K2_SetRelativeLocation` _forwardvision (`KismetMathLibrary.MakeVector` _visiondistance) false false)
  (`BoxComponent.SetBoxExtent` _forwardvision (`KismetMathLibrary.MakeVector` _visiondistance _visiondistance _visiondistance) true))