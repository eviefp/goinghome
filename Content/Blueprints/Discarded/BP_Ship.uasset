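; BP_Ship is the player's physics-driven spaceship, creating debug and dialog HUDs on BeginPlay.
; Input drives paired thrusters for pitch, yaw and roll, impulses for thrust, and projectiles inheriting ship velocity.
; When enabled by bound events, mining line-traces ahead, shrinking asteroids until destroyed.
; Flight, mining and overlaps report to GoingHomeGameState, while Tick orients a cone along velocity.
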(event `InputAction|Shoot`
  (params (Key :type "Key Structure" :default "AnyKey"))
  ;[1 1 1] Shoot
  (:`Released`
    (bind _returnvalue (`|SpawnActorFromClass` "/Game/Blueprints/BP_ShipProjectile.BP_ShipProjectile_C" (`SceneComponent.K2_GetComponentToWorld` (`self.ShootArrow`)) "AdjustIfPossibleButAlwaysSpawn" "OverrideRootScale"))
    (set `/Game/Blueprints/BP_ShipProjectile.ParentActor` self _returnvalue)
    (`PrimitiveComponent.SetPhysicsLinearVelocity` (`/Game/Blueprints/BP_ShipProjectile.Sphere` _returnvalue) (+ (`SceneComponent.GetComponentVelocity` (`self.ShipMesh`)) (* (`SceneComponent.GetForwardVector` (`self.ShootArrow`)) 4000.0)) false "None")))

(event `InputAction|RestartLevel`
  (params (Key :type "Key Structure" :default "AnyKey"))
  (:`Released`
    (bind _returnvalue (`GameplayStatics.GetCurrentLevelName` true))
    (`GameplayStatics.OpenLevel` (`KismetStringLibrary.Conv_StringToName` _returnvalue))))

(event `InputAxis|Pitch`
  (params (AxisValue :type "Float (single-precision)"))
  (bind _pitchup (`self.PitchUp`))
  (bind _pitchdown (`self.PitchDown`))
  (bind _returnvalue (* AxisValue (`self.PitchStrength`)))
  ;[1 1 1] Pitch
  (if (!= AxisValue 0.0)
    (`ActorComponent.Activate` _pitchup false)
    (`ActorComponent.Activate` _pitchdown false)
    (set `PhysicsThrusterComponent.ThrustStrength` _returnvalue _pitchup)
    (set `PhysicsThrusterComponent.ThrustStrength` _returnvalue _pitchdown)
    (bind _asgoing_home_game_state (cast `GoingHomeGameState` (`GameplayStatics.GetGameState`)))
    (`GoingHomeGameState.OnPitch` _asgoing_home_game_state AxisValue)
    (else
      (`ActorComponent.Deactivate` _pitchup)
      (`ActorComponent.Deactivate` _pitchdown))))

(event `self.ReceiveBeginPlay`
  (bind _returnvalue (`GameplayStatics.GetPlayerController` 0))
  ;[1 1 1] BeginPlay
  (`PlayerController.SetViewTargetWithBlend` _returnvalue self 0.0 "VTBlend_Linear" 0.0 false)
  (bind _returnvalue_2 (`|CreateWidget` "/Game/Blueprints/HUD/BP_HUD_Debug.BP_HUD_Debug_C" _returnvalue))
  (`UserWidget.AddToViewport` _returnvalue_2 0)
  (bind _returnvalue_3 (`|CreateWidget` "/Game/Blueprints/HUD/BP_HUD_Dialog.BP_HUD_Dialog_C" _returnvalue))
  (`UserWidget.AddToViewport` _returnvalue_3 0)
  (set `self.CanMine` false)
  (add `self.EnableMining` (delegate `CustomEvent_0`))
  (add `self.DisableMining` (delegate `CustomEvent_1`)))

(event `CustomEvent_0`
  ;[1 1 1] BeginPlay
  (set `self.CanMine` true))

(event `CustomEvent_1`
  ;[1 1 1] BeginPlay
  (set `self.CanMine` false))

(event `InputAxis|Yaw`
  (params (AxisValue :type "Float (single-precision)"))
  (bind _yawright (`self.YawRight`))
  (bind _yawleft (`self.YawLeft`))
  (bind _returnvalue (* AxisValue (`self.YawStrength`)))
  ;[1 1 1] Yaw
  (if (!= AxisValue 0.0)
    (`ActorComponent.Activate` _yawright false)
    (`ActorComponent.Activate` _yawleft false)
    (set `PhysicsThrusterComponent.ThrustStrength` _returnvalue _yawright)
    (set `PhysicsThrusterComponent.ThrustStrength` _returnvalue _yawleft)
    (bind _asgoing_home_game_state (cast `GoingHomeGameState` (`GameplayStatics.GetGameState`)))
    (`GoingHomeGameState.OnYaw` _asgoing_home_game_state AxisValue)
    (else
      (`ActorComponent.Deactivate` _yawright)
      (`ActorComponent.Deactivate` _yawleft))))

(event `self.ReceiveTick`
  (params (DeltaSeconds :type "Float (single-precision)"))
  (bind _shipmesh (`self.ShipMesh`))
  (bind _cone (`self.Cone`))
  ;[1 1 1] Tick - Buttplug
  (bind _returnvalue (`PrimitiveComponent.GetPhysicsLinearVelocity` _shipmesh "None"))
  (`SceneComponent.K2_SetWorldRotation` _cone (`KismetMathLibrary.MakeRotator` (.roll (`KismetMathLibrary.FindLookAtRotation` (`SceneComponent.K2_GetComponentLocation` _cone) (+ (* _returnvalue 100.0) (`SceneComponent.K2_GetComponentLocation` _shipmesh)))) (+ (.pitch (`KismetMathLibrary.FindLookAtRotation` (`SceneComponent.K2_GetComponentLocation` _cone) (+ (* _returnvalue 100.0) (`SceneComponent.K2_GetComponentLocation` _shipmesh)))) -90.0) (.yaw (`KismetMathLibrary.FindLookAtRotation` (`SceneComponent.K2_GetComponentLocation` _cone) (+ (* _returnvalue 100.0) (`SceneComponent.K2_GetComponentLocation` _shipmesh))))) false false))

(event `InputAxis|Roll`
  (params (AxisValue :type "Float (single-precision)"))
  (bind _rollforward (`self.RollForward`))
  (bind _rollbackwards (`self.RollBackwards`))
  (bind _returnvalue (* AxisValue (`self.RollSpeetrength`)))
  ;[1 1 1] Roll
  (if (!= AxisValue 0.0)
    (`ActorComponent.Activate` _rollforward false)
    (`ActorComponent.Activate` _rollbackwards false)
    (set `PhysicsThrusterComponent.ThrustStrength` _returnvalue _rollforward)
    (set `PhysicsThrusterComponent.ThrustStrength` _returnvalue _rollbackwards)
    (bind _asgoing_home_game_state (cast `GoingHomeGameState` (`GameplayStatics.GetGameState`)))
    (`GoingHomeGameState.OnRoll` _asgoing_home_game_state AxisValue)
    (else
      (`ActorComponent.Deactivate` _rollforward)
      (`ActorComponent.Deactivate` _rollbackwards))))

(event `InputAxis|Mine`
  (params (AxisValue :type "Float (single-precision)"))
  (bind _returnvalue (`SceneComponent.K2_GetComponentLocation` (`self.ShipMesh`)))
  ;[1 1 1] Mining
  (if (and (>= AxisValue 1.0) (`self.CanMine`))
    (bind _outhit (`KismetSystemLibrary.LineTraceSingle` _returnvalue (+ _returnvalue (* (`SceneComponent.GetForwardVector` (`self.ForwardArrow`)) 500.0)) "TraceTypeQuery1"))
    (bind (_bblockinghit _binitialoverlap _time _location _impactpoint _normal _impactnormal _physmat _hitactor) (`GameplayStatics.BreakHitResult` _outhit))
    (bind _asbp_mineable_asteroid (cast `/Game/Blueprints/Objects/BP_MineableAsteroid` _hitactor))
    (`GameplayStatics.SpawnEmitterAtLocation` "/Game/Blueprints/BP_MiningParticleEmitter.BP_MiningParticleEmitter" _location (`KismetMathLibrary.FindLookAtRotation` _location (+ _returnvalue (* (`SceneComponent.GetRightVector` (`self.ForwardArrow`)) 5.0))))
    (bind _asgoing_home_game_state (cast `GoingHomeGameState` (`GameplayStatics.GetGameState`)))
    (bind _returnvalue_2 (`KismetStringLibrary.Conv_StringToName` (`KismetSystemLibrary.GetDisplayName` _hitactor)))
    (`GoingHomeGameState.OnMine` _asgoing_home_game_state _returnvalue_2)
    (bind _returnvalue_3 (- (`self.GetActorScale3D` _asbp_mineable_asteroid) (* 0.2 (`GameplayStatics.GetWorldDeltaSeconds`))))
    (`self.SetActorScale3D` _asbp_mineable_asteroid _returnvalue_3)
    (if (<= (.x _returnvalue_3) 0.2)
      (`GoingHomeGameState.OnMineDestroyed` _asgoing_home_game_state _returnvalue_2)
      (`self.K2_DestroyActor` _asbp_mineable_asteroid))))

(event `InputAxis|Thrust`
  (params (AxisValue :type "Float (single-precision)"))
  ;[1 1 1] Thrust
  (`PrimitiveComponent.AddImpulse` (`self.ShipMesh`) (* (`KismetMathLibrary.GetForwardVector` (`SceneComponent.K2_GetComponentRotation` (`self.ForwardArrow`))) (* AxisValue (`self.ThrusterStrength`))) "None" false)
  (bind _asgoing_home_game_state (cast `GoingHomeGameState` (`GameplayStatics.GetGameState`)))
  (`GoingHomeGameState.OnThrust` _asgoing_home_game_state AxisValue))

(event `self.ShipMesh.OnComponentBeginOverlap`
  (params (OverlappedComponent :type "PrimitiveComponent Object Reference") (OtherActor :type "Actor Object Reference") (OtherComp :type "PrimitiveComponent Object Reference") (OtherBodyIndex :type Integer) (bFromSweep :type Boolean) (SweepResult :type "HitResult Structure (by ref)"))
  ;[1 1 1] Overlap Event
  (bind _asgoing_home_game_state (cast `GoingHomeGameState` (`GameplayStatics.GetGameState`)))
  (`GoingHomeGameState.OnOverlap` _asgoing_home_game_state (`KismetStringLibrary.Conv_StringToName` (`KismetSystemLibrary.GetDisplayName` OtherActor))))

(fn `UserConstructionScript`)