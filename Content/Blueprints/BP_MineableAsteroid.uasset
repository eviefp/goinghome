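; BP_MineableAsteroid is an asteroid actor that marks a zone where a player ship can mine.
; When a BP_Ship enters its sphere collision, it calls EnableMining on that ship, and calls DisableMining when the ship leaves.
; The asteroid only toggles the ship's mining state; its graph holds no resource or mining logic of its own.
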(event `self.SphereCollision.OnComponentBeginOverlap`
  (params (OverlappedComponent :type "PrimitiveComponent Object Reference") (OtherActor :type "Actor Object Reference") (OtherComp :type "PrimitiveComponent Object Reference") (OtherBodyIndex :type Integer) (bFromSweep :type Boolean) (SweepResult :type "HitResult Structure (by ref)"))
  (bind _asbp_ship (cast `/Game/Blueprints/BP_Ship` OtherActor))
  (`/Game/Blueprints/BP_Ship.EnableMining` _asbp_ship))

(event `self.SphereCollision.OnComponentEndOverlap`
  (params (OverlappedComponent :type "PrimitiveComponent Object Reference") (OtherActor :type "Actor Object Reference") (OtherComp :type "PrimitiveComponent Object Reference") (OtherBodyIndex :type Integer))
  (bind _asbp_ship (cast `/Game/Blueprints/BP_Ship` OtherActor))
  (`/Game/Blueprints/BP_Ship.DisableMining` _asbp_ship))

(fn `UserConstructionScript`
  (`parent.UserConstructionScript`))