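; OverlapTester is a debug Blueprint, kept in the Discarded folder, that reports overlaps on its Box component.
; When an overlap begins, it formats a message naming itself, its overlapped component, the other actor and that actor's component, then prints it with PrintString.
; It has no construction logic and does not handle the end of an overlap.
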(event `self.Box.OnComponentBeginOverlap`
  (params (OverlappedComponent :type "PrimitiveComponent Object Reference") (OtherActor :type "Actor Object Reference") (OtherComp :type "PrimitiveComponent Object Reference") (OtherBodyIndex :type Integer) (bFromSweep :type Boolean) (SweepResult :type "HitResult Structure (by ref)"))
  (`KismetSystemLibrary.PrintString` (`KismetTextLibrary.Conv_TextToString` (`|FormatText` (`KismetTextLibrary.Conv_StringToText` (`KismetSystemLibrary.GetDisplayName` self)) "Actor {self} : {selfComponent} overlapping with {other} : {otherComponent}" (`KismetTextLibrary.Conv_StringToText` (`KismetSystemLibrary.GetDisplayName` OverlappedComponent)) (`KismetTextLibrary.Conv_StringToText` (`KismetSystemLibrary.GetDisplayName` OtherActor)) (`KismetTextLibrary.Conv_StringToText` (`KismetSystemLibrary.GetDisplayName` OtherComp))))))

(fn `UserConstructionScript`)