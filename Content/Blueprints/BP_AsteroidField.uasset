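; BP_AsteroidField is an asteroid field that scatters randomly chosen actors around its own location when play begins.
; A loop driven by SpawnActors picks classes from Actors, placing each along a random unit vector within MaxDistance.
; Each gets a rotation from a random positive X vector and independent per-axis scale between MinScale and MaxScale.
; Spawns always succeed, adjusting for collision if possible, then attach to the field with KeepRelative rules and welding.
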(event `self.ReceiveBeginPlay`
  (bind _actors (`self.Actors`))
  (bind _returnvalue (`KismetMathLibrary.RandomFloatInRange` (`self.MinScale`) (`self.MaxScale`)))
  ;[1 1 1] Create asteroids
  (for _ (range (+ (`self.SpawnActors`) 1))
    (bind _returnvalue_2 (`|SpawnActorFromClass` (`KismetArrayLibrary.Array_Get` _actors (`KismetMathLibrary.RandomIntegerInRange` 0 (- (`KismetArrayLibrary.Array_Length` _actors) 1))) (`KismetMathLibrary.MakeTransform` (+ (* (`KismetMathLibrary.RandomUnitVector`) (`KismetMathLibrary.RandomFloatInRange` 0.0 (`self.MaxDistance`))) (`self.K2_GetActorLocation` self)) (`KismetMathLibrary.Conv_VectorToRotator` (`KismetMathLibrary.MakeVector` (`KismetMathLibrary.RandomFloatInRange` 0.0 360.0) (`KismetMathLibrary.RandomFloatInRange` 0.0 360.0) (`KismetMathLibrary.RandomFloatInRange` 0.0 360.0))) (`KismetMathLibrary.MakeVector` _returnvalue _returnvalue _returnvalue)) "AdjustIfPossibleButAlwaysSpawn" "OverrideRootScale"))
    (`self.K2_AttachToActor` _returnvalue_2 self "None" "KeepRelative" "KeepRelative" "KeepRelative" true)))

(fn `UserConstructionScript`)