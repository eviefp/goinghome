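; BP_ShipProjectile is a physics-driven projectile, named for ships, that reports what it hits to the game state.
; SetLinearVelocity sets the Sphere's physics velocity, and getter and setter functions track the ParentActor that serves as shooter.
; On a Sphere hit, it passes shooter and victim to GoingHomeGameState's OnProjectileHit and destroys itself, printing a debug string if the cast fails.
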(event `self.Sphere.OnComponentHit`
  (params (HitComponent :type "PrimitiveComponent Object Reference") (OtherActor :type "Actor Object Reference") (OtherComp :type "PrimitiveComponent Object Reference") (NormalImpulse :type "Vector Structure") (Hit :type "HitResult Structure (by ref)"))
  (bind _asgoing_home_game_state (cast `GoingHomeGameState` (`GameplayStatics.GetGameState`))
    (:`then`
      (`GoingHomeGameState.OnProjectileHit` _asgoing_home_game_state (`self.ParentActor`) OtherActor)
      (`self.K2_DestroyActor`))
    (:`CastFailed`
      (`KismetSystemLibrary.PrintString` "bad"))))

(event `self.SetLinearVelocity`
  (params (velocity :type "Vector Structure (by ref)"))
  (`PrimitiveComponent.SetPhysicsLinearVelocity` (`self.Sphere`) velocity false "None"))

(fn `GetProjectileParent`
  (returns (ReturnValue :type "Actor Object Reference"))
  (return (`self.ParentActor`)))

(fn `SetProjectileParent`
  (params (parent :type "Actor Object Reference"))
  (returns (ReturnValue :type Boolean))
  (set `self.ParentActor` parent)
  (return true))

(fn `UserConstructionScript`)